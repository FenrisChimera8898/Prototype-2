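; Laundry basket quest item that the player can carry, inspect and store in the inventory.
; While an item is held, sphere overlaps freeze the mesh and drive Activate or Deactivate by IsBackwards, with paired DoOnce gates preventing repeats.
; Tick watches for R during inspection to add it to inventory, re-armed by Dropped.
; Partial adds keep the remainder; full adds teleport it to the DeathBox before delayed destruction.
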(event OnComponentBeginOverlap(Sphere)
  (params (OverlappedComponent :type Primitive%20Component%20Object%20Reference) (OtherActor :type Actor%20Object%20Reference) (OtherComp :type Primitive%20Component%20Object%20Reference) (OtherBodyIndex :type Integer) (bFromSweep :type Boolean) (SweepResult :type Hit%20Result%20Structure%20%28by%20ref%29))
  (bind _isbackwards (Variables|Default|GetisBackwards))
  (bind _staticmesh (Variables|Default|GetStaticMesh))
  (bind _asfirst_person_character (Utilities|Casting|CastToFirstPersonCharacter (Game|GetPlayerCharacter 0)))
  (if (Variables|/Game/FirstPersonBP/Blueprints/FirstPersonCharacter.FirstPersonCharacter_C|GetPickedUp _asfirst_person_character)
    (Development|PrintString (Utilities|GetDisplayName OtherComp))
    (Physics|SetSimulatePhysics _staticmesh false)
    (Collision|SetCollisionEnabled _staticmesh "QueryOnly")
    (if (not (Physics|IsSimulatingPhysics OtherComp "None"))
      (Utilities|FlowControl|Sequence
        (:then_0
          (Utilities|FlowControl|DoOnce false
            (:Completed
              (if _isbackwards
                (CallFunction|Activate)
                (else
                  (CallFunction|Deactivate))))))
        (:then_1
          (Utilities|FlowControl|DoOnce false) ; enters at Reset
        )))))

(event OnComponentEndOverlap(Sphere)
  (params (OverlappedComponent :type Primitive%20Component%20Object%20Reference) (OtherActor :type Actor%20Object%20Reference) (OtherComp :type Primitive%20Component%20Object%20Reference) (OtherBodyIndex :type Integer))
  (bind _isbackwards (Variables|Default|GetisBackwards))
  (bind _asfirst_person_character (Utilities|Casting|CastToFirstPersonCharacter (Game|GetPlayerCharacter 0)))
  (if (Variables|/Game/FirstPersonBP/Blueprints/FirstPersonCharacter.FirstPersonCharacter_C|GetPickedUp _asfirst_person_character)
    (Utilities|FlowControl|Sequence
      (:then_0
        (Utilities|FlowControl|DoOnce false) ; enters at Reset
      )
      (:then_1
        (Utilities|FlowControl|DoOnce false
          (:Completed
            (if _isbackwards
              (CallFunction|Activate)
              (else
                (CallFunction|Deactivate)))))))))

(event Custom|Dropped
  (Utilities|FlowControl|DoOnce false) ; enters at Reset
)

(event EventBeginPlay
  (bind _output_get (Variables|Default|SetScaleOBJ (Transformation|GetWorldScale (Variables|Default|GetStaticMesh))))
  (Variables|Default|SetgetScale _output_get))

(event EventTick
  (params (DeltaSeconds :type Float%20%28single-precision%29))
  (|CallParentFunction 0.0)
  (bind _asfirst_person_character (Utilities|Casting|CastToFirstPersonCharacter (Game|GetPlayerCharacter 0)))
  (if (and (Variables|/Game/FirstPersonBP/Blueprints/FirstPersonCharacter.FirstPersonCharacter_C|GetPressedR _asfirst_person_character) (== (Variables|/Game/FirstPersonBP/Blueprints/FirstPersonCharacter.FirstPersonCharacter_C|GetInspectObj _asfirst_person_character) self))
    (Utilities|FlowControl|DoOnce false
      (:Completed
        (Utilities|IsValid (Variables|/Game/FirstPersonBP/Blueprints/FirstPersonCharacter.FirstPersonCharacter_C|GetInventoryRef _asfirst_person_character)
          (:Is%20Valid
            (bind (_success_ _rest) (Default|AddItem (Variables|/Game/FirstPersonBP/Blueprints/FirstPersonCharacter.FirstPersonCharacter_C|GetInventoryRef _asfirst_person_character) (Variables|Components|GetItemToAdd) (Variables|Default|GetAmount)))
            (if _success_
              (if (> _rest 0)
                (Variables|Default|SetAmount _rest)
                (else
                  (Variables|/Game/FirstPersonBP/Blueprints/FirstPersonCharacter.FirstPersonCharacter_C|SetAddedToInv _asfirst_person_character true)
                  (Utilities|FlowControl|Delay 0.1)
                  (Variables|/Game/FirstPersonBP/Blueprints/FirstPersonCharacter.FirstPersonCharacter_C|SetAddedToInv _asfirst_person_character false)
                  (bind _asdeath_box (Utilities|Casting|CastToDeathBoxClass "/Game/World/Systems/Inspection/DeathBox.DeathBox_C"))
                  (bind _returnvalue (Actor|GetActorOfClass _asdeath_box))
                  (Transformation|Teleport (Transformation|GetActorLocation _returnvalue) "0, 0, 0")
                  (Default|Endwid _asfirst_person_character)
                  (Utilities|FlowControl|Delay 1e+01)
                  (Actor|DestroyActor))))))))))

(fn ConstructionScript
  (|CallParentFunction))