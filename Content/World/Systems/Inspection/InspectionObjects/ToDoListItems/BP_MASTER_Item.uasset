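; Master item Blueprint for to-do list objects that handles using an inventory item, including toothpaste, milk, cereal and a bowl.
; EventOnUse branches on the item's category; toothpaste goes through the inventory's ToothpasteUsed check, while milk and cereal set local flags.
; A full bowl, or both flags set (once only), records progress on bellaplayercontroller.
; Used items are removed from the inventory by index, and the actor destroys itself when removal succeeds.
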(event Custom|EventOnUse
  (bind _s_iteminfo (Variables|Default|Gets_ItemInfo))
  (bind _category (Utilities|Struct|BreakS_ItemInfos _s_iteminfo))
  (if (Utilities|Enum|Equal(Enum) _category "NewEnumerator2")
    (bind _success_ (Default|ToothpasteUsed (Variables|Default|GetInventory) (Variables|OnSpawn|GetIndex) 1))
    (if _success_
      (bind _success__2 (Default|RemoveItematIndex (Variables|Default|GetInventory) (Variables|OnSpawn|GetIndex) 1))
      (if _success__2
        (Actor|DestroyActor)))
    (else
      (if (Utilities|Enum|Equal(Enum) _category "NewEnumerator5")
        (Variables|Default|SetCerealUsed true))
      (if (Utilities|Enum|Equal(Enum) _category "NewEnumerator4")
        (Variables|Default|SetMilkUsed true))
      (if (Utilities|Enum|Equal(Enum) _category "NewEnumerator7")
        (bind _asbellaplayercontroller (Utilities|Casting|CastTobellaplayercontroller (Game|GetPlayerController 0)))
        (Variables|/Game/FirstPersonBP/Maps/bellaTest/bellaplayercontroller.bellaplayercontroller_C|SetFullBowlEaten? _asbellaplayercontroller true)
        (bind _success__3 (Default|RemoveItematIndex (Variables|Default|GetInventory) (Variables|OnSpawn|GetIndex) 1 :!label _label))
        (if _success__3
          (Actor|DestroyActor))
        (elif (and (Variables|Default|GetCerealUsed) (Variables|Default|GetMilkUsed))
          (Utilities|FlowControl|DoOnce false
            (:Completed
              (bind _asbellaplayercontroller_2 (Utilities|Casting|CastTobellaplayercontroller (Game|GetPlayerController 0)))
              (Variables|/Game/FirstPersonBP/Maps/bellaTest/bellaplayercontroller.bellaplayercontroller_C|SetMilkAndCerealUsed _asbellaplayercontroller_2 true)
              (goto _label)))
          (else
            (bind _success__4 (Default|RemoveItematIndex (Variables|Default|GetInventory) (Variables|OnSpawn|GetIndex) 1))
            (if _success__4
              (Actor|DestroyActor))))))))

(fn ConstructionScript)