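; Inspectable water bottle item that the player can add to the inventory for the to-do list.
; Tick polls for R pressed while this bottle is inspected, firing a DoOnce that Dropped resets.
; It adds the item, keeping any remainder; otherwise it sets WaterBottleFound on the player controller and refreshes the checklist.
; The collected bottle then teleports to the DeathBox, calls the character's Endwid and destroys itself after a delay.
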(event Custom|Dropped
  (Utilities|FlowControl|DoOnce false) ; enters at Reset
)

(event EventBeginPlay
  (Variables|Default|SetScaleOBJ (Transformation|GetWorldScale (Variables|Default|GetStaticMesh))))

(event EventTick
  (params (DeltaSeconds :type Float%20%28single-precision%29))
  (|CallParentFunction 0.0)
  (bind _asfirst_person_character (Utilities|Casting|CastToFirstPersonCharacter (Game|GetPlayerCharacter 0)))
  (if (and (Variables|/Game/FirstPersonBP/Blueprints/FirstPersonCharacter.FirstPersonCharacter_C|GetPressedR _asfirst_person_character) (== (Variables|/Game/FirstPersonBP/Blueprints/FirstPersonCharacter.FirstPersonCharacter_C|GetInspectObj _asfirst_person_character) self))
    (Utilities|FlowControl|DoOnce false
      (:Completed
        (Utilities|IsValid (Variables|/Game/FirstPersonBP/Blueprints/FirstPersonCharacter.FirstPersonCharacter_C|GetInventoryRef _asfirst_person_character)
          (:Is%20Valid
            (bind (_success_ _rest) (Default|AddItem (Variables|/Game/FirstPersonBP/Blueprints/FirstPersonCharacter.FirstPersonCharacter_C|GetInventoryRef _asfirst_person_character) (Variables|Components|GetItemToAdd) (Variables|Default|GetAmount)))
            (if _success_
              (if (> _rest 0)
                (Variables|Default|SetAmount _rest)
                (else
                  (Variables|/Game/FirstPersonBP/Blueprints/FirstPersonCharacter.FirstPersonCharacter_C|SetAddedToInv _asfirst_person_character true)
                  (bind _asbellaplayercontroller (Utilities|Casting|CastTobellaplayercontroller (Game|GetPlayerController 0)))
                  (Variables|/Game/FirstPersonBP/Maps/bellaTest/bellaplayercontroller.bellaplayercontroller_C|SetWaterBottleFound _asbellaplayercontroller true)
                  (bind _asbp_inventory (Utilities|Casting|CastToBP_InventoryClass "/Game/World/Systems/InventorySystemStuff/Blueprints/BP_Inventory.BP_Inventory_C"))
                  (bind _returnvalue (Actor|GetActorOfClass _asbp_inventory))
                  (Default|ChecktheList _returnvalue)
                  (Utilities|FlowControl|Delay 0.1)
                  (Variables|/Game/FirstPersonBP/Blueprints/FirstPersonCharacter.FirstPersonCharacter_C|SetAddedToInv _asfirst_person_character false)
                  (bind _asdeath_box (Utilities|Casting|CastToDeathBoxClass "/Game/World/Systems/Inspection/DeathBox.DeathBox_C"))
                  (bind _returnvalue_2 (Actor|GetActorOfClass _asdeath_box))
                  (Transformation|Teleport (Transformation|GetActorLocation _returnvalue_2) "0, 0, 0")
                  (Default|Endwid _asfirst_person_character)
                  (Utilities|FlowControl|Delay 1e+01)
                  (Actor|DestroyActor))))))))))

(fn ConstructionScript
  (|CallParentFunction))