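; Portal door that teleports the first-person character to its paired PortalBP on hit, working in both directions.
; A hit disables input, then searches all portals for the matching PortalIndex with the opposite Entrance flag and moves the character to its ExitRef.
; Timelines drive the FadeCOL Radius parameter to fade out and in, with delays chained from their Update pins.
; The construction script positions Portal and ExitRef from variables.
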(event Collision|EventHit
  (params (MyComp :type Primitive%20Component%20Object%20Reference) (Other :type Actor%20Object%20Reference) (OtherComp :type Primitive%20Component%20Object%20Reference) (bSelfMoved :type Boolean) (HitLocation :type Vector :default "0, 0, 0") (HitNormal :type Vector :default "0, 0, 0") (NormalImpulse :type Vector :default "0, 0, 0") (Hit :type Hit%20Result%20Structure%20%28by%20ref%29))
  (bind _asfirst_person_character (Utilities|Casting|CastToFirstPersonCharacter Other))
  (Development|PrintString "Sound plays" true true "(R=1.000000,G=0.151122,B=0.352119,A=1.000000)" 0.05)
  (if (Variables|Default|GetEntrance?)
    (Input|DisableInput _asfirst_person_character 0)
    (bind _fadeout (Timeline|Fadeout1 PlayFromStart)
      (:Update
        (Rendering|Material|SetScalarParameterValue "/Game/World/PortalDoors/FadeCOL.FadeCOL" "Radius" _fadeout :!class /Script/Engine.KismetMaterialLibrary)
        (Utilities|FlowControl|Delay 1.0)
        (bind _outactors (Actor|GetAllActorsOfClass "PortalBP_C"))
        (bind _array_element (Utilities|Array|ForEachLoopwithBreak _outactors :!label _label)
          (:LoopBody
            (if (and (== (Variables|PortalBP_C|GetPortalIndex _array_element) (Variables|Default|GetPortalIndex)) (not (Variables|PortalBP_C|GetEntrance? _array_element)))
              (goto _label Break)))
          (:Completed
            (Transformation|SetActorLocation _asfirst_person_character (Transformation|GetWorldLocation (Variables|PortalBP_C|GetExitRef _array_element)) false false)
            (bind _fadein (Timeline|Fadein1 PlayFromStart)
              (:Update
                (Rendering|Material|SetScalarParameterValue "/Game/World/PortalDoors/FadeCOL.FadeCOL" "Radius" _fadein :!class /Script/Engine.KismetMaterialLibrary)
                (Utilities|FlowControl|Delay 1.0)
                (Input|EnableInput _asfirst_person_character 0)))))))
    (else
      (Input|DisableInput _asfirst_person_character 0)
      (bind _fadeout_2 (Timeline|Fadeout2 PlayFromStart)
        (:Update
          (Rendering|Material|SetScalarParameterValue "/Game/World/PortalDoors/FadeCOL.FadeCOL" "Radius" _fadeout_2 :!class /Script/Engine.KismetMaterialLibrary)
          (Utilities|FlowControl|Delay 1.0)
          (bind _outactors_2 (Actor|GetAllActorsOfClass "PortalBP_C"))
          (bind _array_element_2 (Utilities|Array|ForEachLoopwithBreak _outactors_2 :!label _label_2)
            (:LoopBody
              (if (and (== (Variables|PortalBP_C|GetPortalIndex _array_element_2) (Variables|Default|GetPortalIndex)) (and (not (Variables|Default|GetEntrance?)) (Variables|PortalBP_C|GetEntrance? _array_element_2)))
                (goto _label_2 Break)))
            (:Completed
              (Transformation|SetActorLocation _asfirst_person_character (Transformation|GetWorldLocation (Variables|PortalBP_C|GetExitRef _array_element_2)) false false)
              (bind _fadein_2 (Timeline|Fadein2 PlayFromStart)
                (:Update
                  (Rendering|Material|SetScalarParameterValue "/Game/World/PortalDoors/FadeCOL.FadeCOL" "Radius" _fadein_2 :!class /Script/Engine.KismetMaterialLibrary)
                  (Utilities|FlowControl|Delay 1.0)
                  (Input|EnableInput _asfirst_person_character 0))))))))))

(fn ConstructionScript
  ;[1 1 1] Set portal and exit
  (Transformation|SetRelativeTransform (Variables|Default|GetPortal) (Variables|Default|GetPortalTransform) false false)
  (Transformation|SetRelativeLocation (Variables|Default|GetExitRef) (Variables|Default|GetExitLocation) false false))