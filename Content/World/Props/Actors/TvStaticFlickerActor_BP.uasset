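; TV static flicker prop actor that blinks a cube on and off at irregular intervals with positional static audio.
; BeginPlay starts the Flicker event, which alternates the cube's visibility after random delays and calls itself to loop indefinitely.
; Each visibility change plays the Static sound at the cube's location with shared attenuation, and the reappearing step also reassigns it to Static_Cue.
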(event Custom|flicker
  (bind _returnvalue (Math|Random|RandomFloatinRange 0.1 3.0))
  (bind _cube (Variables|Default|GetCube))
  (Utilities|FlowControl|Delay _returnvalue)
  (Rendering|SetVisibility _cube false false)
  (Audio|PlaySoundatLocation (Variables|Default|GetStatic) (Transformation|GetWorldLocation (Variables|Default|GetCube)) "0, 0, 0" 1.0 1.0 0.0 "/Game/World/Audio/GoodMorningSounds/GMSoundAttenuation_SA.GMSoundAttenuation_SA" 0 0)
  (Utilities|FlowControl|Delay _returnvalue)
  (Rendering|SetVisibility _cube true false)
  (CallFunction|Flicker)
  (Variables|Default|SetStatic "/Game/World/Audio/GoodMorningSounds/Static_Cue.Static_Cue")
  (Audio|PlaySoundatLocation (Variables|Default|GetStatic) (Transformation|GetWorldLocation (Variables|Default|GetCube)) "0, 0, 0" 1.0 1.0 0.0 "/Game/World/Audio/GoodMorningSounds/GMSoundAttenuation_SA.GMSoundAttenuation_SA" 0 0))

(event EventBeginPlay
  (CallFunction|Flicker)
  (Variables|Default|SetStatic (Variables|Default|GetStatic)))

(event Collision|EventActorBeginOverlap
  (params (OtherActor :type Actor%20Object%20Reference)))

(event EventTick
  (params (DeltaSeconds :type Float%20%28single-precision%29)))

(fn ConstructionScript)