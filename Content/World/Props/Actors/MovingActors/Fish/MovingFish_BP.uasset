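; Fish prop actor that moves along the spline of a referenced track actor, using cart-named variables and logic.
; On BeginPlay, if ActiveCart is set, the CartMover timeline plays in reverse from its end at a rate derived from Duration.
; Each update maps Alpha to spline distance and applies that world location and rotation.
; CartStartOffset sets the timeline time just before ReverseFromEnd, which restarts it from the end.
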(event Custom|MoveCart
  (bind _trackref (Variables|Default|GetTrackRef))
  (bind _spline (Variables|/Game/World/Props/Actors/MovingActors/Fish/FishTrack_BP.FishTrack_BP_C|GetSpline _trackref))
  (Components|Timeline|SetPlayRate (Variables|Default|GetCartMover) (/ 1.0 (Variables|Default|GetDuration)))
  (Components|Timeline|SetNewTime (Variables|Default|GetCartMover) (Variables|Default|GetCartStartOffset))
  (bind _alpha (Timeline|CartMover ReverseFromEnd)
    (:Update
      (Variables|Default|SetAlpha _alpha)
      (Transformation|SetActorLocationAndRotation (Spline|GetLocationatDistanceAlongSpline _spline (Math|Float|Lerp 0.0 (Spline|GetSplineLength (Variables|/Game/World/Props/Actors/MovingActors/Fish/FishTrack_BP.FishTrack_BP_C|GetSpline (Variables|Default|GetTrackRef))) (Variables|Default|GetAlpha)) "World") (Spline|GetRotationatDistanceAlongSpline _spline (Math|Float|Lerp 0.0 (Spline|GetSplineLength (Variables|/Game/World/Props/Actors/MovingActors/Fish/FishTrack_BP.FishTrack_BP_C|GetSpline (Variables|Default|GetTrackRef))) (Variables|Default|GetAlpha)) "World")))))

(event EventBeginPlay
  (if (Variables|Default|GetActiveCart)
    (CallFunction|MoveCart)))

(fn ConstructionScript)